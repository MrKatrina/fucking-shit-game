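; Stairs trigger box for the Subway level that slows the player while they are inside it.
; Overlap begin and end cast the actor to FirstPersonCharacter and set CharacterMovement MaxWalkSpeed to a reduced value, then back to a fixed walking speed.
; An unconnected key-check attempt at a faster speed is left in the graph and never runs.
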(event Collision|EventActorBeginOverlap
  (params (OtherActor :type Actor%20Object%20Reference))
  ;[1 1 1] main shit
  (bind _asfirst_person_character (Utilities|Casting|CastToFirstPersonCharacter OtherActor))
  (Variables|/Script/Engine.CharacterMovementComponent|SetMaxWalkSpeed (Variables|/Script/Engine.Character|GetCharacterMovement _asfirst_person_character) 3.5e+02))

(event Collision|EventActorEndOverlap
  (params (OtherActor :type Actor%20Object%20Reference))
  ;[1 1 1] main shit
  (bind _asfirst_person_character (Utilities|Casting|CastToFirstPersonCharacter OtherActor))
  (Variables|/Script/Engine.CharacterMovementComponent|SetMaxWalkSpeed (Variables|/Script/Engine.Character|GetCharacterMovement _asfirst_person_character) 4.5e+02))

(event Input|ActionEvents|InputActionSprint
  (params (Key :type Key%20Structure))
  ;[1 1 1] shitty attempt
)

(fn ConstructionScript)