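; Subway card sign Blueprint that reveals a widget and a set of companion components while the player is nearby.
; BeginPlay caches the FirstPersonCharacter and hides them all.
; Box overlap begin and end by that player toggle their visibility and the CanInteract flag.
; The face-player logic is inactive: the spin event is empty, and the looping timer and yaw-only look-at rotation on PFB never run.
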(event OnComponentBeginOverlap(Box)
  (params (OverlappedComponent :type Primitive%20Component%20Object%20Reference) (OtherActor :type Actor%20Object%20Reference) (OtherComp :type Primitive%20Component%20Object%20Reference) (OtherBodyIndex :type Integer) (bFromSweep :type Boolean) (SweepResult :type Hit%20Result%20Structure%20%28by%20ref%29))
  (if (== OtherActor (Variables|Default|GetPlayer%20ref))
    (Variables|Default|Setcan%20interact true)
    (Rendering|SetVisibility (Variables|Default|GetWidget1) true false)))

(event OnComponentEndOverlap(Box)
  (params (OverlappedComponent :type Primitive%20Component%20Object%20Reference) (OtherActor :type Actor%20Object%20Reference) (OtherComp :type Primitive%20Component%20Object%20Reference) (OtherBodyIndex :type Integer))
  (if (== OtherActor (Variables|Default|GetPlayer%20ref))
    (Variables|Default|Setcan%20interact false)
    (Rendering|SetVisibility (Variables|Default|GetWidget1) false false)))

(event Custom|spin
  ;[1 1 1] text_follow player
)

(event EventBeginPlay
  ;[1 1 1] text_follow player
  (bind _asfirst_person_character (Utilities|Casting|CastToFirstPersonCharacter (Game|GetPlayerCharacter 0)))
  (Variables|Default|SetPlayer%20ref _asfirst_person_character)
  (Rendering|SetVisibility (Variables|Default|GetWidget1) false false))

(fn ConstructionScript)